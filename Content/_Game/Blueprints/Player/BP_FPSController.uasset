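; Player controller for a team-based FPS that handles team selection, pawn spawning and local UI.
; A delayed client event shows the team widget; attacker or defender picks go through server events to the game mode's spawn requests.
; SpawnPlayer spawns and possesses the character, then restores game-only input on the client.
; It also relays health, ammo, weapon icon, crosshair recoil and camera shake updates, and toggles the buy menu.
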(event `self.ReceiveBeginPlay`
  ;[1 1 1] get the GM referecnce after clients join the server
  (bind _asbp_base_game_mode (cast `/Game/_Game/Blueprints/GameMode_BP/BP_BaseGameMode` (`GameplayStatics.GetGameMode`)))
  (set `self.BaseGameMode` _asbp_base_game_mode)
  (`self.GetGameRule`))

(event `GetGameRule`
  ;[1 1 1] get the GM referecnce after clients join the server
  (bind _gamerule (`/Game/_Game/Blueprints/GameMode_BP/BP_BaseGameMode.F_GameRules` (`self.BaseGameMode`)))
  (set `self.Game Rule` _gamerule))

(event `/Game/_Game/Blueprints/Interfaces/INT_PlayerController.ShowTeamSelection`
  ;[1 1 1] brings up team selection widget
  (`KismetSystemLibrary.Delay` 1.0)
  (`self.Client_ShowTeamSelection`))

(event `Client_ShowTeamSelection`
  ;[1 1 1] brings up team selection widget
  (bind _returnvalue (`|CreateWidget` "/Game/_Game/UI/Widget/W_SelectTeam.W_SelectTeam_C"))
  (bind _output_get (set `self.W_TeamSelection` _returnvalue))
  (`UserWidget.AddToViewport` _output_get 0)
  (`WidgetBlueprintLibrary.SetInputMode_GameAndUIEx` self (`self.W_TeamSelection`))
  (set `self.bShowMouseCursor` true))

(event `/Game/_Game/Blueprints/Interfaces/INT_PlayerController.AttackerSelect`
  ;[1 1 1] Spawn attackers or defenders
  (`Widget.RemoveFromParent` (`self.W_TeamSelection`))
  (`self.Server_SpawnAttacker`))

(event `Server_SpawnAttacker`
  ;[1 1 1] Spawn attackers or defenders
  (`/Game/_Game/Blueprints/GameMode_BP/BP_BaseGameMode.RequestAttackerSpawn` (`self.BaseGameMode`) self "/Game/_Game/Blueprints/Player/Attacker_Character.Attacker_Character_C"))

(event `/Game/_Game/Blueprints/Interfaces/INT_PlayerController.DefenderSelect`
  ;[1 1 1] Spawn attackers or defenders
  (`Widget.RemoveFromParent` (`self.W_TeamSelection`))
  (`self.Server_SpawnDefender`))

(event `Server_SpawnDefender`
  ;[1 1 1] Spawn attackers or defenders
  (`/Game/_Game/Blueprints/GameMode_BP/BP_BaseGameMode.RequestDefenderSpawn` (`self.BaseGameMode`) self "/Game/_Game/Blueprints/Player/Defender_Character.Defender_Character_C"))

(event `/Game/_Game/Blueprints/Interfaces/INT_PlayerController.SpawnPlayer`
  (params (player :type "/Game/_Game/Blueprints/Player/BP_BaseCharacter Class Reference") (transform :type "Transform Structure"))
  ;[1 1 1] Spawn attackers or defenders
  (bind _returnvalue (`|SpawnActorFromClass` player transform "AdjustIfPossibleButAlwaysSpawn" "OverrideRootScale" null null))
  (bind _output_get (set `self.PLayerChar` _returnvalue))
  (`self.Possess` _output_get)
  (`self.Client_HideMouse`))

(event `Client_HideMouse`
  ;[1 1 1] Spawn attackers or defenders
  (`WidgetBlueprintLibrary.SetInputMode_GameOnly` self)
  (set `self.bShowMouseCursor` false))

(event `/Game/_Game/Blueprints/Interfaces/INT_PlayerController.CreatePLayerUI`
  ;[1 1 1] Create UI
  (if (`self.IsLocalPlayerController`)
    (bind _returnvalue (`|CreateWidget` "/Game/_Game/UI/Widget/W_PlayerUI.W_PlayerUI_C"))
    (bind _output_get (set `self.W_PlayerUI` _returnvalue))
    (`UserWidget.AddToViewport` _output_get 0)))

(event `/Game/_Game/Blueprints/Interfaces/INT_PlayerController.UpdateHealthUI`
  (params (NewHealth :type "Float (single-precision)") (IncomingDamage :type "Float (single-precision)"))
  ;[1 1 1] Create UI
  (`/Game/_Game/UI/Widget/W_PlayerUI.UpdateHealth` (`self.W_PlayerUI`) (`KismetMathLibrary.Round` NewHealth) (`KismetMathLibrary.Round` IncomingDamage)))

(event `/Game/_Game/Blueprints/Interfaces/INT_PlayerController.DoCrosshairRecoil`
  ;[1 1 1] Create UI
  (`/Game/_Game/UI/Widget/W_PlayerUI.CrosshairRecoil` (`self.W_PlayerUI`)))

(event `/Game/_Game/Blueprints/Interfaces/INT_PlayerController.Update Current Ammo UI`
  (params (CurrentAmmo :type Integer))
  ;[1 1 1] Create UI
  (`/Game/_Game/UI/Widget/W_PlayerUI.UpdateCurrentAmmo` (`self.W_PlayerUI`) CurrentAmmo))

(event `/Game/_Game/Blueprints/Interfaces/INT_PlayerController.ShowAmmoOverlay`
  (params (Show :type Boolean))
  ;[1 1 1] Create UI
  (`/Game/_Game/UI/Widget/W_PlayerUI.ShowHideAmmoOverlay` (`self.W_PlayerUI`) Show))

(event `/Game/_Game/Blueprints/Interfaces/INT_PlayerController.UpdateMaxAmmoUI`
  (params (TotalAmmoLeft :type Integer))
  ;[1 1 1] Create UI
  (`/Game/_Game/UI/Widget/W_PlayerUI.UpdateAmmoLeft` (`self.W_PlayerUI`) TotalAmmoLeft))

(event `/Game/_Game/Blueprints/Interfaces/INT_PlayerController.Death`)

(event `/Game/_Game/Blueprints/Interfaces/INT_PlayerController.BuyMenuUI`
  (params (Attacker :type Boolean))
  (if (not (`self.BuyMenuOpen`))
    (`self.W_BuyMenu`
      (:`then`
        _)
      (:`else`
        (bind _returnvalue (`|CreateWidget` "/Game/_Game/BuyMenu/BuyMenu.BuyMenu_C"))
        (set `self.W_BuyMenu` _returnvalue)))
    (`UserWidget.AddToViewport` (`self.W_BuyMenu`) 0)
    (set `self.BuyMenuOpen` true)
    (else
      (bind _w_buymenu (`self.W_BuyMenu`)
        (:`then`
          (`Widget.RemoveFromParent` _w_buymenu)
          (set `self.BuyMenuOpen` false))
        (:`else`)))))

(event `/Game/_Game/Blueprints/Interfaces/INT_PlayerController.PlayCameraShake`
  (params (CameraShake :type "MatineeCameraShake Class Reference"))
  (`self.ClientStartCameraShake` CameraShake))

(event `/Game/_Game/Blueprints/Interfaces/INT_PlayerController.UpdateWeaponIcon`
  (params (Icon :type "Texture2D Object Reference"))
  (`/Game/_Game/UI/Widget/W_PlayerUI.UpdateWeaponIcon` (`self.W_PlayerUI`) Icon))

(fn `UserConstructionScript`)