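; Third-person weapon actor that serves as a world pickup and holds the weapon's type, ammo info and shooting effects.
; On server overlap, a player with a free primary or secondary slot receives it via interface messages, and its physics and collision switch off.
; Dropping restores physics with an impulse, re-enabling pickup after a delay.
; Effects skip the local pawn's weapon; firing is stubbed as moved to base character, leaving body-part hitscan damage unwired.
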(event `self.ReceiveBeginPlay`
  (bind _weaponinfo (`self.WeaponInfo`))
  (bind ((`MaxAmmoInGun_76_463583B442DF3A8EEBF1A1A6FA0E29B6` _maxammoingun) (`MaxAmmoInClip_77_51778431447D81997D68D18E8BA83712` _maxammoinclip)) (break `/Game/_Game/Blueprints/Struct/S_WeaponInfo` _weaponinfo))
  (setmembers `/Game/_Game/Blueprints/Struct/S_WeaponInfo` :`StructRef` _weaponinfo :`CurrentAmmoInGun` _maxammoingun :`CurrentAmmoInClip` _maxammoinclip))

(event `self.Sphere.OnComponentBeginOverlap`
  (params (OverlappedComponent :type "PrimitiveComponent Object Reference") (OtherActor :type "Actor Object Reference") (OtherComp :type "PrimitiveComponent Object Reference") (OtherBodyIndex :type Integer) (bFromSweep :type Boolean) (SweepResult :type "HitResult Structure (by ref)"))
  (bind _weaponinfo (`self.WeaponInfo`))
  (`/Engine/EditorBlueprintResources/ActorMacros.Switch Has Authority`
    (:`Authority`
      (if (`self.ActorHasTag` OtherActor "Player")
        (switch `/Game/_Game/Blueprints/Weapon/E_WeaponType` (`self.WeaponType`)
          (:`NewEnumerator0`
            (bind _hasprimary (message `/Game/_Game/Blueprints/Interfaces/INT_BaseCharacter.CheckForPrimary` OtherActor))
            (if (not _hasprimary)
              (`self.EquipWeapon`)
              (message `/Game/_Game/Blueprints/Interfaces/INT_BaseCharacter.EquipPrimary` OtherActor _weaponinfo self)))
          (:`NewEnumerator1`
            (bind _hassecondary (message `/Game/_Game/Blueprints/Interfaces/INT_BaseCharacter.CheckForSecondary` OtherActor))
            (if (not _hassecondary)
              (`self.EquipWeapon`)
              (message `/Game/_Game/Blueprints/Interfaces/INT_BaseCharacter.EquipSecondary` OtherActor _weaponinfo self))))))))

(event `EquipWeapon`
  (bind _weapon (`self.Weapon`))
  (`PrimitiveComponent.SetEnableGravity` _weapon false)
  (`PrimitiveComponent.SetSimulatePhysics` _weapon false)
  (`PrimitiveComponent.SetCollisionEnabled` _weapon "NoCollision")
  (`PrimitiveComponent.SetCollisionEnabled` (`self.Sphere`) "NoCollision"))

(event `UnEquipWeapon`
  (params (Impulse :type "Vector Structure"))
  (bind _weapon (`self.Weapon`))
  (`self.SetOwner` null)
  (`PrimitiveComponent.SetCollisionEnabled` _weapon "QueryAndPhysics")
  (`PrimitiveComponent.SetEnableGravity` _weapon true)
  (`PrimitiveComponent.SetSimulatePhysics` _weapon true)
  (`PrimitiveComponent.AddImpulse` (`self.Weapon`) Impulse "None" false)
  (`KismetSystemLibrary.Delay` 1.0)
  (`PrimitiveComponent.SetCollisionEnabled` (`self.Sphere`) "QueryOnly"))

(event `Server_FireWeapon`
  (params (CameraLocation :type "Vector Structure") (CameraForwardVector :type "Rotator Structure"))
  ;[1 1 1] it has been changed in base character
)

(event `multi_ShootingEffects`
  (if (not (== (`self.GetOwner`) (`GameplayStatics.GetPlayerPawn` 0)))
    (`GameplayStatics.SpawnEmitterAttached` (`self.MuzzleFlash`) (`self.Weapon`) "MuzzleFlash")
    (`GameplayStatics.PlaySoundAtLocation` (`self.FiringSound`) (`self.K2_GetActorLocation`) (struct) 1.0 1.0 0.0 null null null)
    (message `/Game/_Game/Blueprints/Interfaces/INT_PlayerController.PlayCameraShake` (`self.GetInstigatorController`) (`self.CameraShake`))))

(event `UpdateweaponInfo`
  (params (WeaponInfo :type "/Game/_Game/Blueprints/Struct/S_WeaponInfo Structure"))
  (set `self.WeaponInfo` WeaponInfo))

(fn `UserConstructionScript`)