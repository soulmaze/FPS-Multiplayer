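; BP_BaseGameMode is a game mode for an attackers versus defenders game, handling team selection and spawn placement.
; On post-login it tells the new player controller to show team selection, and on begin play it caches all attacker and defender spawn point actors.
; Team spawn requests message the requesting controller to spawn the given player at a randomly chosen cached point's transform.
; A getter exposes the GameRules variable.
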(event `self.K2_PostLogin`
  (params (NewPlayer :type "PlayerController Object Reference"))
  (message `/Game/_Game/Blueprints/Interfaces/INT_PlayerController.ShowTeamSelection` NewPlayer))

(event `self.ReceiveBeginPlay`
  (`|ExecutionSequence`
    (:`then_0`
      (bind _outactors (`GameplayStatics.GetAllActorsOfClass` "/Game/_Game/Blueprints/SpawnPoints/BP_AttackersSpawnPoint.BP_AttackersSpawnPoint_C"))
      (set `self.AttackersSpawnPoints` _outactors))
    (:`then_1`
      (bind _outactors_2 (`GameplayStatics.GetAllActorsOfClass` "/Game/_Game/Blueprints/SpawnPoints/BP_DefendersSpawnPoint.BP_DefendersSpawnPoint_C"))
      (set `self.DefendenrsSpawnPoint` _outactors_2))))

(event `RequestAttackerSpawn`
  (params (PLayerController :type "PlayerController Object Reference") (player :type "/Game/_Game/Blueprints/Player/BP_BaseCharacter Class Reference"))
  (bind _attackersspawnpoints (`self.AttackersSpawnPoints`))
  (message `/Game/_Game/Blueprints/Interfaces/INT_PlayerController.SpawnPlayer` PLayerController player (`self.GetTransform` (`|GetArrayItem` _attackersspawnpoints (`KismetMathLibrary.RandomIntegerInRange` 0 (- (`KismetArrayLibrary.Array_Length` _attackersspawnpoints) 1))))))

(event `RequestDefenderSpawn`
  (params (PLayerController :type "PlayerController Object Reference") (player :type "/Game/_Game/Blueprints/Player/BP_BaseCharacter Class Reference"))
  (bind _defendenrsspawnpoint (`self.DefendenrsSpawnPoint`))
  (message `/Game/_Game/Blueprints/Interfaces/INT_PlayerController.SpawnPlayer` PLayerController player (`self.GetTransform` (`|GetArrayItem` _defendenrsspawnpoint (`KismetMathLibrary.RandomIntegerInRange` 0 (- (`KismetArrayLibrary.Array_Length` _defendenrsspawnpoint) 1))))))

(fn `F_GameRules`
  (returns (GameRule :type "/Game/_Game/Blueprints/Struct/S_GameRules Structure"))
  (return (`self.GameRules`)))

(fn `UserConstructionScript`)